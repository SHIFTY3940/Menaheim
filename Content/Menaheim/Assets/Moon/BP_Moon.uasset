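; BP_Moon is a moon actor that fades its visuals and lighting between day and night states.
; NightTransition plays the DayToNight timeline, driving moon material opacity, glow density, moon light intensity and the FogParams collection's Opacity.
; DayTransition reverses the same timeline to undo the change.
; The construction script points the actor's X axis at an Origin point and applies a uniform Scale.
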(event Custom|Night%20Transition
  (bind (_direction _moon _glow _post_process _moon_light) (Timeline|Day%20To%20Night Play)
    (:Update
      (Rendering|Material|SetScalarParameterValueonMaterials (Variables|Default|GetMoon) "Opacity" _moon)
      (Rendering|Material|SetScalarParameterValueonMaterials (Variables|Default|GetGlow) "Density" _glow)
      (Rendering|Components|Light|SetIntensity (Variables|Default|GetMoon%20LIght) _moon_light)
      (Rendering|Material|SetScalarParameterValue "/Game/Testing_Grounds/Materials/Coloured_Fog/FogParams.FogParams" "Opacity" _post_process :!class /Script/Engine.KismetMaterialLibrary))))

(event Custom|Day%20Transition
  (bind (_direction _moon _glow _post_process _moon_light) (Timeline|Day%20To%20Night Reverse)
    (:Update
      (Rendering|Material|SetScalarParameterValueonMaterials (Variables|Default|GetMoon) "Opacity" _moon)
      (Rendering|Material|SetScalarParameterValueonMaterials (Variables|Default|GetGlow) "Density" _glow)
      (Rendering|Components|Light|SetIntensity (Variables|Default|GetMoon%20LIght) _moon_light)
      (Rendering|Material|SetScalarParameterValue "/Game/Testing_Grounds/Materials/Coloured_Fog/FogParams.FogParams" "Opacity" _post_process :!class /Script/Engine.KismetMaterialLibrary))))

(fn ConstructionScript
  (bind _scale (Variables|Default|GetScale))
  (Transformation|SetActorRotation (Math|Conversions|RotationFromXVector (Math|Vector|Normalize (- (Variables|Default|GetOrigin) (Transformation|GetActorLocation)))))
  (Transformation|SetActorScale3D (Math|Vector|MakeVector _scale _scale _scale)))